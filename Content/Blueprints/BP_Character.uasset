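; First-person player character that picks up, carries and delivers masks, with mouse look and a crosshair widget.
; E line-traces along the camera to attach a BP_Mask to a carry point, or returns the held one to the Backwall sphere tagged with its TargetSocket.
; Space submits that socket to BP_GameState_Jam, destroying the mask on success or returning it on failure, behind a cooldown; K quits.
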(event Input|EnhancedActionEvents|EnhancedInputActionIA_MouseXYZ
  (params (ActionValue :type Vector%202D%20Structure) (ElapsedSeconds :type Float%20%28double-precision%29) (TriggeredSeconds :type Float%20%28double-precision%29) (InputAction :type Input%20Action%20Object%20Reference :default "/Game/Input/IA_MouseXYZ.IA_MouseXYZ"))
  (Pawn|Input|AddControllerYawInput (.x ActionValue))
  (Pawn|Input|AddControllerPitchInput (* (.y ActionValue) -1.0)))

(event EventBeginPlay
  (bind _asbp_controller (Utilities|Casting|CastToBP_Controller (Pawn|GetController)))
  (Utilities|IsValid (PlayerController|LocalPlayerSubsystems|GetEnhancedInputLocalPlayerSubsystem _asbp_controller)
    (:Is%20Valid
      (Input|AddMappingContext (PlayerController|LocalPlayerSubsystems|GetEnhancedInputLocalPlayerSubsystem _asbp_controller) "/Game/Input/IMC_Input.IMC_Input" 0 "(bIgnoreAllPressedKeysUntilRelease=True,bForceImmediately=False,bNotifyUserSettings=False)")
      (bind _returnvalue (UserInterface|CreateWidget "/Game/Blueprints/WBP_Crosshair.WBP_Crosshair_C"))
      (UserInterface|Viewport|AddtoViewport _returnvalue 0))))

(event Input|KeyboardEvents|E
  (params (Key :type Key%20Structure :default "None"))
  (:Pressed
    (if (Variables|Default|GetAreWeHoldingtheObject)
      (CallFunction|DroptheObject (Variables|Default|GetObject%20to%20Carry))
      (else
        (bind _outhit_hitactor (CallFunction|LineTrace))
        (bind _asbp_mask (Utilities|Casting|CastToBP_Mask _outhit_hitactor))
        (CallFunction|CarrytheObject _asbp_mask)))))

(event Input|KeyboardEvents|SpaceBar
  (params (Key :type Key%20Structure :default "None"))
  (bind _object_to_carry (Variables|Default|GetObject%20to%20Carry))
  (:Pressed
    (if (Variables|Default|GetSpaceCheck)
      (Variables|Default|SetSpaceCheck false)
      (bind _asbp_game_state_jam (Utilities|Casting|CastToBP_GameState_Jam (Game|GetGameState)))
      (bind _success (Default|SubmitDeliveredMask _asbp_game_state_jam (Variables|/Game/Blueprints/BP_Mask.BP_Mask_C|GetTargetSocket (Variables|Default|GetObject%20to%20Carry))))
      (if _success
        (Actor|DestroyActor _object_to_carry)
        (Variables|Default|SetAreWeHoldingtheObject false)
        (Utilities|FlowControl|Delay 3.0)
        (Variables|Default|SetSpaceCheck true)
        (else
          (CallFunction|DroptheObject _object_to_carry)
          (Utilities|FlowControl|Delay 3.0)
          (Variables|Default|SetSpaceCheck true))))))

(event Input|KeyboardEvents|K
  (params (Key :type Key%20Structure :default "None"))
  (:Pressed
    (Game|QuitGame 0 "Quit" false)))

(fn ConstructionScript)

(fn LineTrace
  (bind _capsulecomponent (Variables|Collision|GetCapsuleComponent))
  (bind _returnvalue (Transformation|GetWorldLocation _capsulecomponent))
  (bind _outhit (Collision|LineTraceByChannel _returnvalue (+ (* (Math|Vector|GetForwardVector (Variables|Default|GetCamera)) 3e+02) _returnvalue) "TraceTypeQuery1" false 0 "ForDuration"))
  (return (.hitactor _outhit)))

(fn CarrytheObject
  (params (ObjectToCarry :type BP%20Mask%20Object%20Reference))
  (bind _scene (Variables|Default|GetScene))
  (bind _output_get (Variables|Default|SetObject%20to%20Carry ObjectToCarry))
  (Transformation|SetWorldLocation (Variables|/Game/Blueprints/BP_Mask.BP_Mask_C|GetSphere _output_get) (Transformation|GetWorldLocation _scene) false false)
  (Transformation|AttachComponentToComponent (Variables|/Game/Blueprints/BP_Mask.BP_Mask_C|GetSphere _output_get) _scene "None" "KeepWorld" "KeepWorld" "KeepWorld" true)
  (Variables|Default|SetAreWeHoldingtheObject true)
  (Physics|SetSimulatePhysics (Variables|/Game/Blueprints/BP_Mask.BP_Mask_C|GetSphere _output_get) false)
  (Collision|SetCollisionEnabled (Variables|/Game/Blueprints/BP_Mask.BP_Mask_C|GetSphere _output_get) "NoCollision")
  (Default|CallOnItemAttached (Variables|/Game/Blueprints/BP_Mask.BP_Mask_C|GetTargetSocket ObjectToCarry)))

(fn DroptheObject
  (params (Object%20To%20Drop :type BP%20Mask%20Object%20Reference))
  (bind _asbp_mask (Utilities|Casting|CastToBP_Mask Object%20To%20Drop))
  (bind _outactors (Actor|GetAllActorswithTag "Backwall"))
  (for _array_element (Actor|GetComponentsByClass (Utilities|Array|Get(acopy) _outactors) "/Script/Engine.SphereComponent")
    (if (== (Variables|/Game/Blueprints/BP_Mask.BP_Mask_C|GetTargetSocket _asbp_mask) (Utilities|Array|Get(acopy) (Variables|/Script/Engine.ActorComponent|GetComponentTags _array_element)))
      (Transformation|AttachComponentToComponent Object%20To%20Drop _array_element "None" "SnapToTarget" "SnapToTarget" "KeepWorld" true)
      (Collision|SetCollisionEnabled (Variables|/Game/Blueprints/BP_Mask.BP_Mask_C|GetSphere Object%20To%20Drop) "QueryOnly")
      (Variables|Default|SetAreWeHoldingtheObject false)
      (return))))