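; Base customer character that walks to an order point, reacts to the order result, then leaves through the spawner's exit point.
; Tick moves it in straight, unswept steps toward the target while a sine wave bounces its Paper sprite, then fires reached-order or reached-exit calls.
; The game state's order-result event stops movement and starts a fixed delay, identical for success or failure, before exiting.
; Reaching the exit also notifies the CustomerSpawner.
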(event Custom|MoveToOrder
  (params (OrderPoint :type Actor%20Object%20Reference))
  (Variables|Default|SetTargetLoc (Transformation|GetActorLocation OrderPoint))
  (Variables|Default|SetbMoving true)
  (Variables|Default|SetbGoingToExit false))

(event Custom|MoveToExit
  (params (ExitPoint :type Actor%20Object%20Reference))
  (Variables|Default|SetTargetLoc (Transformation|GetActorLocation ExitPoint))
  (Variables|Default|SetbMoving true)
  (Variables|Default|SetbGoingToExit true))

(event Custom|ReactToOrder
  (params (isSuccess :type Boolean))
  (Development|PrintString "ReactOrder")
  (if isSuccess
    (Utilities|FlowControl|Delay 3.0)
    (else
      (Utilities|FlowControl|Delay 3.0)))
  (CallFunction|MovetoExit (Variables|/Game/Blueprints/BP_CustomerSpawner.BP_CustomerSpawner_C|GetExitPoint (Variables|Default|GetCustomerSpawner))))

(event Custom|ReactToResult
  (params (IsSuccess :type Boolean))
  (Variables|Default|SetbMoving false)
  (CallFunction|ReacttoOrder IsSuccess))

(event EventBeginPlay
  (bind _asbp_game_state_jam (Utilities|Casting|CastToBP_GameState_Jam (Game|GetGameState)))
  (EventDispatchers|BindEventtoOnOrderResult _asbp_game_state_jam (delegate Custom|ReactToResult)))

(event EventTick
  (params (DeltaSeconds :type Float%20%28single-precision%29))
  (bind _returnvalue (Transformation|GetActorLocation))
  (bind _targetloc (Variables|Default|GetTargetLoc))
  (bind _papersprite (Variables|Default|GetPaperSprite))
  (if (Variables|Default|GetbMoving)
    (Utilities|FlowControl|Sequence
      (:then_0
        (Transformation|SetActorLocation (+ (* (* (Variables|Default|GetMoveSpeed) DeltaSeconds) (Math|Vector|Normalize (- _targetloc _returnvalue))) _returnvalue) false false)
        (if (< (Math|Vector|Distance(Vector) _returnvalue _targetloc) 2e+01)
          (Transformation|SetActorLocation (Variables|Default|GetTargetLoc) false false)
          (Variables|Default|SetbMoving false)
          (if (Variables|Default|GetbGoingToExit)
            (Default|CallOnReachedExit)
            (Default|HandleCustomerFinished (Variables|Default|GetCustomerSpawner))
            (else
              (Default|CallOnReachedOrder)))))
      (:then_1
        (Utilities|IsValid _papersprite
          (:Is%20Valid
            (Transformation|SetRelativeLocation _papersprite (Math|Vector|MakeVector 0.0 0.0 (* (Math|Float|Absolute(Float) (Math|Trig|Sin(Radians) (* (Variables|Default|GetBounceSpeed) (Utilities|Time|GetGameTimeinSeconds)))) (Variables|Default|GetBounceHeight))) false false)))))
    (else
      (Transformation|SetRelativeLocation _papersprite "0, 0, 0" false false))))

(fn ConstructionScript)