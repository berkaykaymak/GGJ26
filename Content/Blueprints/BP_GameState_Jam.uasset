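; Game state for a jam game that runs customer mask orders and judges deliveries.
; SetCurrentOrder stores the customer scenario, creates a WBP_Dialogue widget and types out the first dialogue line.
; SubmitDeliveredMask compares the delivered mask ID to the scenario's correct one and broadcasts OnOrderResult.
; Its own bound handler types a random success or fail message in the current widget, then removes it after a short delay.
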(event Custom|OnOrderResult_Event
  (params (IsSuccess :type Boolean))
  (bind _currentdialoguewidget (Variables|Default|GetCurrentDialogueWidget))
  (bind _successmessages (Variables|Default|GetSuccessMessages))
  (bind _failmessages (Variables|Default|GetFailMessages))
  (Utilities|IsValid _currentdialoguewidget
    (:Is%20Valid
      (if IsSuccess
        (Default|StartTyping _currentdialoguewidget (Utilities|Array|Get(acopy) _successmessages (Math|Random|RandomIntegerinRange 0 (Utilities|Array|LastIndex _successmessages))))
        (else
          (Default|StartTyping _currentdialoguewidget (Utilities|Array|Get(acopy) _failmessages (Math|Random|RandomIntegerinRange 0 (Utilities|Array|LastIndex _failmessages))))))
      (Utilities|FlowControl|Delay 3.0)
      (Widget|RemovefromParent _currentdialoguewidget))))

(event EventBeginPlay
  (EventDispatchers|BindEventtoOnOrderResult (delegate Custom|OnOrderResult_Event)))

(fn ConstructionScript)

(fn SetCurrentOrder
  (params (NewScenerio :type BP%20Customer%20Scenario%20Data%20Object%20Reference))
  (Development|PrintString (Utilities|String|ToString(Name) (Variables|/Game/Blueprints/BP_CustomerScenario_Data.BP_CustomerScenario_Data_C|GetScenarioID NewScenerio)))
  (bind _output_get (Variables|Default|SetCurrentCustomerScenario NewScenerio))
  (bind _returnvalue (UserInterface|CreateWidget "/Game/Blueprints/WBP_Dialogue.WBP_Dialogue_C"))
  (bind _output_get_2 (Variables|Default|SetCurrentDialogueWidget _returnvalue))
  (UserInterface|Viewport|AddtoViewport _output_get_2 0)
  (Default|StartTyping _output_get_2 (.Dialog (Utilities|Struct|BreakS_DialogueLine (Utilities|Array|Get(acopy) (Variables|/Game/Blueprints/BP_CustomerScenario_Data.BP_CustomerScenario_Data_C|GetDialogueLines _output_get))))))

(fn SubmitDeliveredMask
  (params (DeliveredMaskID :type Name))
  (bind _currentcustomerscenario (Variables|Default|GetCurrentCustomerScenario))
  (bind _correctmaskid (Variables|/Game/Blueprints/BP_CustomerScenario_Data.BP_CustomerScenario_Data_C|GetCorrectMaskID _currentcustomerscenario))
  (bind _returnvalue (== DeliveredMaskID _correctmaskid))
  (Development|PrintString (Utilities|String|Append "Is correct mask: " (Utilities|String|ToString(Boolean) _returnvalue)))
  (if _returnvalue
    (Default|CallOnOrderResult true)
    (else
      (Default|CallOnOrderResult false))))