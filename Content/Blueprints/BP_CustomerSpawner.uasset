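; Customer spawner that runs the game's day-by-day loop of single customers walking in to order and leaving.
; StartDay loads music, customer classes and scenarios from MasterSchedule, then spawns customers sequentially.
; Arrivals pass their scenario to BP_GameState_Jam, optionally ducking music for an arrival sound; its order result sends them to the exit, triggering the next spawn.
; An exhausted list shows a day transition widget, starts the next day and updates the background.
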(event Custom|SpawnNextCustomer
  (Utilities|IsValid (Variables|Default|GetActiveCustomer)
    (:Is%20Valid
      (Development|PrintString "ÖNCEKİ MÜŞTERİ HALA DURUYOR")
      (Actor|DestroyActor (Variables|Default|GetActiveCustomer))
      (Variables|Default|SetActiveCustomer 0))
    (:Is%20Not%20Valid
      _))
  (if (>= (Variables|Default|GetCurrentIndex) (Utilities|Array|Length (Variables|Default|GetCustomerClasses)))
    (bind _result (Math|Integer|IncrementInt (Variables|Default|GetCurrentDayIndex))
      (:%20%20
        (if (< _result (Utilities|Array|Length (Variables|Default|GetMasterSchedule)))
          (bind _returnvalue (UserInterface|CreateWidget "/Game/Blueprints/WBP_DayTransition.WBP_DayTransition_C"))
          (Default|UpdateDayText _returnvalue (Variables|Default|GetCurrentDayIndex))
          (UserInterface|Viewport|AddtoViewport _returnvalue 0)
          (Utilities|FlowControl|Delay 3.0)
          (Development|PrintString "Yeni gün başlıyor")
          (CallFunction|StartDay)
          (Development|PrintString (Utilities|String|Append "Current Day Index:" (Utilities|String|ToString(Integer) (Variables|Default|GetCurrentDayIndex))))
          (Widget|RemovefromParent _returnvalue)
          (Default|UpdateMaterialforDay (Variables|Default|GetBackgroundImage) (Variables|Default|GetCurrentDayIndex))
          (else
            (Development|PrintString "OYUN BİTTİ")))))
    (else
      (bind _returnvalue_2 (Game|SpawnActorfromClass (Utilities|Array|Get(acopy) (Variables|Default|GetCustomerClasses) (Variables|Default|GetCurrentIndex)) (Transformation|GetWorldTransform (Variables|Default|GetArrow)) "Undefined" "MultiplyWithRoot" 0 self (Utilities|Array|Get(acopy) (Variables|Default|GetCustomerScenarios) (Variables|Default|GetCurrentIndex)) 0))
      (bind _output_get (Variables|Default|SetActiveCustomer _returnvalue_2))
      (Default|MovetoOrder _output_get (Variables|Default|GetOrderPoint))
      (EventDispatchers|BindEventtoOnReachedOrder _output_get (delegate Custom|OnCustomerReachedOrder)))))

(event Custom|HandleCustomerFinished
  (Utilities|IsValid (Variables|Default|GetActiveCustomer)
    (:Is%20Valid
      (Actor|DestroyActor (Variables|Default|GetActiveCustomer))
      (Variables|Default|SetActiveCustomer 0)
      (Variables|Default|SetCurrentIndex (+ (Variables|Default|GetCurrentIndex) 1))
      (Utilities|FlowControl|Delay 1.0)
      (CallFunction|SpawnNextCustomer))))

(event Custom|OnCustomerReachedOrder
  (bind _activecustomer (Variables|Default|GetActiveCustomer))
  (bind _myscenario (Variables|/Game/Customers/BP_CustomerCharacter_Base.BP_CustomerCharacter_Base_C|GetMyScenario _activecustomer))
  (Variables|Default|SetisArrived true)
  (bind _asbp_game_state_jam (Utilities|Casting|CastToBP_GameState_Jam (Game|GetGameState)))
  (Default|SetCurrentOrder _asbp_game_state_jam _myscenario)
  (Variables|/Game/Blueprints/BP_GameState_Jam.BP_GameState_Jam_C|SetCurrentCustomer _asbp_game_state_jam _activecustomer)
  (if (Variables|/Game/Customers/BP_CustomerScenario_Data.BP_CustomerScenario_Data_C|GetisOrderSound _myscenario)
    (CallFunction|ControlMusic false)
    (Audio|PlaySound2D (Variables|/Game/Customers/BP_CustomerScenario_Data.BP_CustomerScenario_Data_C|GetArrivalSound _myscenario) 1.0 1.0 0.0 0 0)))

(event Custom|OnCustomerReachedExit
  (CallFunction|HandleCustomerFinished))

(event Custom|HandleResult
  (params (IsSuccess :type Boolean))
  (bind _activecustomer (Variables|Default|GetActiveCustomer))
  (if IsSuccess
    _
    (else
      _))
  (Default|MovetoExit (Variables|Default|GetActiveCustomer) (Variables|Default|GetExitPoint))
  (Utilities|IsValid _activecustomer
    (:Is%20Valid
      (Default|MovetoExit _activecustomer (Variables|Default|GetExitPoint))
      (EventDispatchers|BindEventtoOnReachedExit _activecustomer (delegate Custom|OnCustomerReachedExit)))))

(event Custom|ControlMusic
  (params (Pause :type Boolean))
  (bind _backgroundmusicref (Variables|Default|GetBackgroundMusicRef))
  (Audio|Components|Audio|AdjustVolume _backgroundmusicref 0.0 0.3 "Linear" :!class /Script/Engine.AudioComponent)
  (Utilities|FlowControl|Delay 3.0)
  (Audio|Components|Audio|AdjustVolume _backgroundmusicref 0.0 1.0 "Linear" :!class /Script/Engine.AudioComponent))

(event EventBeginPlay
  (Utilities|FlowControl|Delay 0.2)
  (bind _asbp_game_state_jam (Utilities|Casting|CastToBP_GameState_Jam (Game|GetGameState)))
  (EventDispatchers|BindEventtoOnOrderResult _asbp_game_state_jam (delegate Custom|HandleResult))
  (CallFunction|StartDay))

(fn ConstructionScript)

(fn StartDay
  (bind _masterschedule (Variables|Default|GetMasterSchedule))
  (bind _currentdayindex (Variables|Default|GetCurrentDayIndex))
  (bind _output (Utilities|Array|Get(acopy) _masterschedule _currentdayindex))
  (bind (_dailylist _dayscustomerlist _dailymusic) (Utilities|Struct|BreakS_DaySchedule _output))
  (bind _returnvalue (Audio|SpawnSound2D _dailymusic 1.0 1.0 0.0 0))
  (Variables|Default|SetBackgroundMusicRef _returnvalue)
  (Variables|Default|SetCustomerScenarios _dailylist)
  (Variables|Default|SetCustomerClasses _dayscustomerlist)
  (Variables|Default|SetCurrentIndex 0)
  (CallFunction|SpawnNextCustomer))